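; In-world armory menu that lets the hero pick a weapon from display slots and puts the currently held one back in its place.
; While open, it shows ArmoryHUD, walks the player to HeroPosition and ramps up pointing at the selected weapon.
; Axis input moves a pointer between occupied slots and Jump equips.
; Dagger and spear are placed on BeginPlay, but only sword and hammer are selectable.
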(event `self.ReceiveBeginPlay`
  (bind _swordobject (`self.SwordObject`))
  (bind _swordslot (`self.SwordSlot`))
  (bind _hammerobject (`self.HammerObject`))
  (bind _hammerslot (`self.hammerSlot`))
  (bind _daggerobject (`self.DaggerObject`))
  (bind _daggerslot (`self.DaggerSlot`))
  (bind _spearobject (`self.SpearObject`))
  (bind _spearslot (`self.SpearSlot`))
  (bind _outactors (`GameplayStatics.GetAllActorsOfClass` "/Game/Robin/Hero/HeroCharacterBP.HeroCharacterBP_C"))
  (set `self.Player` (`KismetArrayLibrary.Array_Get` _outactors))
  (bind _returnvalue (`|CreateWidget` "/Game/Robin/Menus/ArmoryHUD.ArmoryHUD_C"))
  (bind _output_get (set `self.HUDReference` _returnvalue))
  (set `/Game/Robin/Menus/ArmoryHUD.Armatory` self _output_get)
  (`Widget.SetVisibility` _output_get "Hidden")
  (`UserWidget.AddToViewport` _output_get 0)
  (if (!= _swordobject null)
    (`SceneComponent.K2_SetWorldLocationAndRotation` (`SkeletalMeshActor.SkeletalMeshComponent` _swordobject) (`SceneComponent.K2_GetComponentLocation` _swordslot) (`SceneComponent.K2_GetComponentRotation` _swordslot) false true))
  (if (!= _hammerobject null)
    (`SceneComponent.K2_SetWorldLocationAndRotation` (`SkeletalMeshActor.SkeletalMeshComponent` _hammerobject) (`SceneComponent.K2_GetComponentLocation` _hammerslot) (`SceneComponent.K2_GetComponentRotation` _hammerslot) false false))
  (if (!= _daggerobject null)
    (`SceneComponent.K2_SetWorldLocationAndRotation` (`SkeletalMeshActor.SkeletalMeshComponent` _daggerobject) (`SceneComponent.K2_GetComponentLocation` _daggerslot) (`SceneComponent.K2_GetComponentRotation` _daggerslot) false true))
  (if (!= _spearobject null)
    (`SceneComponent.K2_SetWorldLocationAndRotation` (`SkeletalMeshActor.SkeletalMeshComponent` _spearobject) (`SceneComponent.K2_GetComponentLocation` _spearslot) (`SceneComponent.K2_GetComponentRotation` _spearslot) false true)))

(event `AdjustPointer`
  ;[1 1 1] Adjust the pointer to the selected weapon
  (`SceneComponent.K2_SetWorldLocation` (`self.Pointer`) (`KismetMathLibrary.MakeVector` (.x (`SceneComponent.K2_GetComponentLocation` (select `/Game/Robin/WeaponType` (`self.WeaponSlot`) :`NewEnumerator0` (`self.hammerSlot`) :`NewEnumerator1` (`self.SwordSlot`)))) (.y (`SceneComponent.K2_GetComponentLocation` (`self.Pointer`))) (.z (`SceneComponent.K2_GetComponentLocation` (select `/Game/Robin/WeaponType` (`self.WeaponSlot`) :`NewEnumerator0` (`self.hammerSlot`) :`NewEnumerator1` (`self.SwordSlot`))))) false true)
  (bind _weapon (`self.Get Selected Weapon`))
  (bind _output_get (set `self.SelectedWeapon` _weapon))
  (set `/Game/Robin/Hero/HeroCharacterBP.Target` _output_get (`self.Player`)))

(event `self.MoveRight`
  (params (`Axis Value` :type "Float (single-precision)"))
  ;[1 1 1] Read Input
  (if (> `Axis Value` 0.5)
    (`/Engine/EditorBlueprintResources/StandardMacros.DoOnce` false :!label _label
      (:`Completed`
        (`self.WeaponToRight`)))
    (else
      (`|ExecutionSequence`
        (:`then_0`
          (goto _label :!via `Reset`))
        (:`then_1`
          (if (< `Axis Value` -0.5)
            (`/Engine/EditorBlueprintResources/StandardMacros.DoOnce` false :!label _label_2
              (:`Completed`
                (`self.WeaponToLeft`)))
            (else
              (goto _label_2 :!via `Reset`))))))))

(event `self.Exit`
  (params (Pressed :type Boolean) (Key :type "Key Structure" :default "AnyKey"))
  ;[1 1 1] Read Input
  (`self.CloseArmatory`))

(event `self.Jump`
  (params (Pressed :type Boolean) (Key :type "Key Structure" :default "AnyKey"))
  ;[1 1 1] Read Input
  (if Pressed
    (`/Engine/EditorBlueprintResources/StandardMacros.DoOnce` false :!label _label_3
      (:`Completed`
        (`self.SelectWeapon`)))
    (else
      (goto _label_3 :!via `Reset`))))

(event `WeaponToRight`
  ;[1 1 1] Got to the next/previous weapon
  (set `self.WeaponSlot` (select `/Game/Robin/WeaponType` (`self.WeaponSlot`) :`NewEnumerator2` "NewEnumerator1" :`NewEnumerator0` "NewEnumerator1" :`NewEnumerator1` "NewEnumerator0" :!type "/Game/Robin/WeaponType Enum") :!label _label_4)
  (if (== (select `/Game/Robin/WeaponType` (`self.WeaponSlot`) :`NewEnumerator0` (`self.HammerObject`) :`NewEnumerator1` (`self.SwordObject`)) null)
    (goto _label_4)
    (else
      (`self.AdjustPointer` :!label _label_5))))

(event `OpenArmatory`
  (bind _player (`self.Player`))
  ;[1 1 1] Open/Close Armatory
  (`Widget.SetVisibility` (`self.HUDReference`) "Visible")
  (set `/Game/Robin/Hero/HeroCharacterBP.InMenu` true _player)
  (set `/Game/Robin/Hero/HeroCharacterBP.Menu` self _player)
  (set `self.WeaponSlot` "NewEnumerator2")
  (`self.WeaponToRight`))

(event `WeaponToLeft`
  ;[1 1 1] Got to the next/previous weapon
  (set `self.WeaponSlot` (select `/Game/Robin/WeaponType` (`self.WeaponSlot`) :`NewEnumerator2` "NewEnumerator1" :`NewEnumerator0` "NewEnumerator1" :`NewEnumerator1` "NewEnumerator0" :!type "/Game/Robin/WeaponType Enum") :!label _label_6)
  (if (== (select `/Game/Robin/WeaponType` (`self.WeaponSlot`) :`NewEnumerator0` (`self.HammerObject`) :`NewEnumerator1` (`self.SwordObject`)) null)
    (goto _label_6)
    (else
      (goto _label_5))))

(event `CloseArmatory`
  (bind _player (`self.Player`))
  ;[1 1 1] Open/Close Armatory
  (`Widget.SetVisibility` (`self.HUDReference`) "Hidden")
  (set `/Game/Robin/Hero/HeroCharacterBP.InMenu` false _player)
  (set `/Game/Robin/Hero/HeroCharacterBP.Menu` null _player)
  (set `/Game/Robin/Hero/HeroCharacterBP.PointAtTarget` 0.0 _player)
  (set `/Game/Robin/Hero/HeroCharacterBP.Target` null _player))

(event `SelectWeapon`
  (bind _weapon (`/Game/Robin/Hero/HeroCharacterBP.Weapon` (`self.Player`)))
  (bind _weapontype (`/Game/Blueprints/WeaponType.WeaponType` _weapon))
  (bind _returnvalue (select `/Game/Robin/WeaponType` _weapontype :`NewEnumerator0` (`self.hammerSlot`) :`NewEnumerator1` (`self.SwordSlot`)))
  ;[1 1 1] Equip the selected weapon
  ;;[1 1 1] Take the weapon out of the armatory
  (switch `/Game/Robin/WeaponType` (`self.WeaponSlot`)
    (:`NewEnumerator0`
      (set `self.HammerObject` null))
    (:`NewEnumerator1`
      (set `self.SwordObject` null)))
  ;;[1 1 1] Take the weapon from the player in the armatory
  (if (!= _weapon null)
    (`self.DetachRootComponentFromParent` _weapon true)
    (switch `/Game/Robin/WeaponType` _weapontype
      (:`NewEnumerator0`
        (set `self.HammerObject` _weapon))
      (:`NewEnumerator1`
        (set `self.SwordObject` _weapon)))
    (`self.K2_SetActorLocationAndRotation` _weapon (`SceneComponent.K2_GetComponentLocation` _returnvalue) (`SceneComponent.K2_GetComponentRotation` _returnvalue) false true)
    (set `self.WeaponSlot` _weapontype)
    ;;[1 1 1] Give the player the weapon
    (`/Game/Robin/Hero/HeroCharacterBP.SelectNewWeapon` (`self.Player`) (`self.SelectedWeapon`))
    (else
      (`/Game/Robin/Hero/HeroCharacterBP.SelectNewWeapon` (`self.Player`) (`self.SelectedWeapon`))))
  (if (== (select `/Game/Robin/WeaponType` (`self.WeaponSlot`) :`NewEnumerator0` (`self.HammerObject`) :`NewEnumerator1` (`self.SwordObject`)) null)
    (`self.CloseArmatory`)
    (else
      (`self.WeaponToRight`))))

(event `self.ReceiveTick`
  (params (DeltaSeconds :type "Float (single-precision)"))
  (bind _player (`self.Player`))
  (bind _heroposition (`self.HeroPosition`))
  (bind _player_2 (`self.Player`))
  (bind _returnvalue (`KismetMathLibrary.MakeVector` (.x (`SceneComponent.K2_GetComponentLocation` _heroposition)) (.y (`SceneComponent.K2_GetComponentLocation` _heroposition))))
  (bind _returnvalue_2 (`KismetMathLibrary.MakeVector` (.x (`SceneComponent.K2_GetComponentLocation` (`Character.CapsuleComponent` _player))) (.y (`SceneComponent.K2_GetComponentLocation` (`Character.CapsuleComponent` _player)))))
  (if (== (`/Game/Robin/Hero/HeroCharacterBP.Menu` _player) self)
    (if (> (`KismetMathLibrary.VSize` (- _returnvalue_2 _returnvalue)) 10.0)
      (`Pawn.AddMovementInput` _player_2 (`KismetMathLibrary.GetDirectionVector` _returnvalue_2 _returnvalue) 1.0 false)
      (goto _label_7 :!via `Reset`)
      (else
        (`|ExecutionSequence`
          (:`then_0`
            (`/Engine/EditorBlueprintResources/StandardMacros.DoOnce` false :!label _label_7
              (:`Completed`
                (`self.SetActorRotation` _player_2 (`SceneComponent.K2_GetComponentRotation` _heroposition)))))
          (:`then_1`
            _))
        (set `/Game/Robin/Hero/HeroCharacterBP.PointAtTarget` (`KismetMathLibrary.FMin` (+ (/ DeltaSeconds (`self.PointAtTargetTime`)) (`/Game/Robin/Hero/HeroCharacterBP.PointAtTarget` _player_2)) 1.0) _player_2)))))

(fn `Get Selected Weapon`
  (returns (Weapon :type "/Game/Blueprints/WeaponType Object Reference"))
  (return (select `/Game/Robin/WeaponType` (`self.WeaponSlot`) :`NewEnumerator0` (`self.HammerObject`) :`NewEnumerator1` (`self.SwordObject`))))

(fn `UserConstructionScript`)