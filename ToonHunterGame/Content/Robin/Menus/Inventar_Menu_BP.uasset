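; In-world 3D inventory menu for the hero, laying items on a chest's rotated grid and pairing it with an InventarHUD widget.
; Opening blends to the player's menu camera and spawns a gold item from the player's gold count.
; DoOnce-gated axis input steps a wrapping index that moves the pointer and sets the player's target.
; Tick opens or closes the chest and ramps the player's point-at-target value while the menu is active.
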(event `self.ReceiveBeginPlay`
  ;[1 1 1] Get Player
  (bind _outactors (`GameplayStatics.GetAllActorsOfClass` "/Game/Robin/Hero/HeroCharacterBP.HeroCharacterBP_C"))
  (set `self.Player` (`KismetArrayLibrary.Array_Get` _outactors))
  ;[1 1 1] Create HUD
  (bind _returnvalue (`|CreateWidget` "/Game/Robin/Menus/InventarHUD.InventarHUD_C"))
  (bind _output_get (set `self.HUDReference` _returnvalue))
  (set `/Game/Robin/Menus/InventarHUD.Inventar` self _output_get)
  (`Widget.SetVisibility` _output_get "Hidden")
  (`UserWidget.AddToViewport` _output_get 0)
  ;[1 1 1] Set item position
  (for (_ _array_index) (`self.ItemList`)
    (`self.GetPosition` _array_index)))

(event `self.OpenMenu`
  (`PlayerController.SetViewTargetWithBlend` (`GameplayStatics.GetPlayerController` 0) (`/Game/Robin/Hero/HeroCharacterBP.MenuCamera` (`self.Player`)) 0.5 "VTBlend_Linear" 0.0 true)
  (`self.OpenInventar`))

(event `AdjustPointer`
  (bind _item (`KismetArrayLibrary.Array_Get` (`self.ItemList`) (`self.Index`)))
  ;[1 1 1] Adjust Pointer
  (bind _position (`self.GetPosition` (`self.Index`)))
  (`SceneComponent.K2_SetWorldLocation` (`self.Pointer`) _position false true)
  (if (!= _item null)
    (set `/Game/Robin/Hero/HeroCharacterBP.Target` (`ActorComponent.GetOwner` _item) (`self.Player`))))

(event `OpenInventar`
  ;[1 1 1] Open/Close Menu
  (`self.Update Inventar`)
  (`Widget.SetVisibility` (`self.HUDReference`) "Visible")
  (set `/Game/Robin/Hero/HeroCharacterBP.InMenu` true (`self.Player`))
  (`self.AdjustPointer`))

(event `PlaceItems`
  ;[1 1 1] Place Items
  (for (_array_element _array_index) (`self.ItemList`)
    (bind _position (`self.GetPosition` _array_index))
    (`self.K2_SetActorLocation` (`ActorComponent.GetOwner` _array_element) _position false true)))

(event `CloseInventar`
  ;[1 1 1] Open/Close Menu
  (set `/Game/Robin/Hero/HeroCharacterBP.PointAtTarget` 0.0 (`self.Player`))
  (`Widget.SetVisibility` (`self.HUDReference`) "Hidden")
  (set `/Game/Robin/Hero/HeroCharacterBP.InMenu` false (`self.Player`)))

(event `ItemLeft`
  (bind _returnvalue (`KismetArrayLibrary.Array_Length` (`self.ItemList`)))
  ;[1 1 1] Menu Navigation
  (set `self.Index` (mod (- (+ (`self.Index`) _returnvalue) 1) _returnvalue))
  (`self.AdjustPointer` :!label _label))

(event `Update Inventar`
  (if (> (`/Game/Robin/Hero/HeroCharacterBP.Amount_Gold` (`self.Player`)) 0)
    (bind _position (`self.GetPosition` 0))
    (bind _returnvalue (`|SpawnActorFromClass` "/Game/Gold_Item.Gold_Item_C" (`KismetMathLibrary.MakeTransform` _position (struct) (0.2 0.2 0.2)) "Undefined" "OverrideRootScale"))
    (bind _item (`/Game/Gold_Item.Item` _returnvalue))
    (set `/Game/Robin/Item.Count` (`/Game/Robin/Hero/HeroCharacterBP.Amount_Gold` (`self.Player`)) _item)
    (`KismetArrayLibrary.Array_Set` (`self.ItemList`) 0 _item)))

(event `ItemRight`
  ;[1 1 1] Menu Navigation
  (set `self.Index` (mod (+ (`self.Index`) 1) (`KismetArrayLibrary.Array_Length` (`self.ItemList`))))
  (goto _label))

(event `ItemDown`
  (bind _returnvalue (`KismetArrayLibrary.Array_Length` (`self.ItemList`)))
  ;[1 1 1] Menu Navigation
  (set `self.Index` (mod (- (+ (`self.Index`) _returnvalue) (`self.MaxColumns`)) _returnvalue))
  (goto _label))

(event `ItemUp`
  ;[1 1 1] Menu Navigation
  (set `self.Index` (mod (+ (`self.Index`) (`self.MaxColumns`)) (`KismetArrayLibrary.Array_Length` (`self.ItemList`))))
  (goto _label))

(event `self.ReceiveTick`
  (params (DeltaSeconds :type "Float (single-precision)"))
  (bind _player (`self.Player`))
  (bind _player_2 (`self.Player`))
  (bind _player_3 (`self.Player`))
  (bind _chest (`self.Chest`))
  (if (and (== (`/Game/Robin/Hero/HeroCharacterBP.Menu` _player_3) self) (`/Game/Robin/Hero/HeroCharacterBP.InMenu` _player_3))
    (`/Game/Blueprints/Menu/Inventory.Open` _chest DeltaSeconds)
    (else
      (`/Game/Blueprints/Menu/Inventory.Close` _chest DeltaSeconds)))
  (if (`/Game/Robin/Hero/HeroCharacterBP.InMenu` _player)
    (if (== (`/Game/Robin/Hero/HeroCharacterBP.Menu` _player) self)
      (set `/Game/Robin/Hero/HeroCharacterBP.PointAtTarget` (`KismetMathLibrary.FMin` (+ (/ DeltaSeconds (`self.PointAtTargetTime`)) (`/Game/Robin/Hero/HeroCharacterBP.PointAtTarget` _player_2)) 1.0) _player_2))))

(event `self.MoveUp`
  (params (`Axis Value` :type "Float (single-precision)"))
  ;[1 1 1] Read Input
  (if (> `Axis Value` 0.5)
    (`/Engine/EditorBlueprintResources/StandardMacros.DoOnce` false :!label _label_2
      (:`Completed`
        (`self.ItemUp`)))
    (else
      (`|ExecutionSequence`
        (:`then_0`
          (goto _label_2 :!via `Reset`))
        (:`then_1`
          (if (< `Axis Value` -0.5)
            (`/Engine/EditorBlueprintResources/StandardMacros.DoOnce` false :!label _label_3
              (:`Completed`
                (`self.ItemDown`)))
            (else
              (goto _label_3 :!via `Reset`))))))))

(event `self.MoveRight`
  (params (`Axis Value` :type "Float (single-precision)"))
  ;[1 1 1] Read Input
  (if (< `Axis Value` -0.5)
    (`/Engine/EditorBlueprintResources/StandardMacros.DoOnce` false :!label _label_4
      (:`Completed`
        (`self.ItemRight`)))
    (else
      (`|ExecutionSequence`
        (:`then_0`
          (goto _label_4 :!via `Reset`))
        (:`then_1`
          (if (> `Axis Value` 0.5)
            (`/Engine/EditorBlueprintResources/StandardMacros.DoOnce` false :!label _label_5
              (:`Completed`
                (`self.ItemLeft`)))
            (else
              (goto _label_5 :!via `Reset`))))))))

(event `self.Exit`
  (params (Pressed :type Boolean) (Key :type "Key Structure" :default "AnyKey"))
  ;[1 1 1] Read Input
  (`self.CloseInventar`))

(fn `GetPosition`
  (params (index :type Integer))
  (returns (position :type "Vector Structure"))
  (bind _rasterground (`self.RasterGround`))
  (bind _maxcolumns (`self.MaxColumns`))
  (bind (_min _max) (`StaticMeshComponent.GetLocalBounds` _rasterground))
  (bind _returnvalue (- _max _min))
  (return (+ (`SceneComponent.K2_GetComponentLocation` (`self.DefaultSceneRoot`)) (`KismetMathLibrary.GreaterGreater_VectorRotator` (+ (`KismetMathLibrary.MakeVector` (* (mod index _maxcolumns) (/ (* (.x (`SceneComponent.RelativeScale3D` _rasterground)) (.x _returnvalue)) (`KismetMathLibrary.Conv_IntToDouble` (`self.MaxColumns`)))) (* (/ index _maxcolumns) (/ (* (.y (`SceneComponent.RelativeScale3D` _rasterground)) (.y _returnvalue)) (`KismetMathLibrary.Conv_IntToDouble` (`self.MaxRows`))))) (`KismetMathLibrary.MakeVector` (* (.x (/ _returnvalue -2.0)) (.x (`SceneComponent.RelativeScale3D` _rasterground))) (* (.y (/ _returnvalue -2.0)) (.y (`SceneComponent.RelativeScale3D` _rasterground))))) (`self.K2_GetActorRotation`)))))

(fn `GetSelectedItem`
  (returns (Item :type "/Game/Robin/Item Object Reference"))
  (return (`KismetArrayLibrary.Array_Get` (`self.ItemList`) (`self.Index`))))

(fn `UserConstructionScript`
  (`parent.UserConstructionScript`)
  (`KismetArrayLibrary.Array_Resize` (`self.ItemList`) (* (`self.MaxRows`) (`self.MaxColumns`))))