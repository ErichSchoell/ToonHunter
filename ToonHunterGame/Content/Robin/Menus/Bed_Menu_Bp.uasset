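; Bed menu actor that moves the hero onto the bed's spot and lets them toggle sleeping.
; OpenMenu flags the hero as in-menu and blends the view to the hero's MenuCamera.
; While this is the active menu, Tick walks the hero to the root in XY, using DoOnce to align rotation on arrival.
; Jump toggles Sleeping, leaving the menu on waking, and Exit clears both states, neither checking the active menu.
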(event `self.ReceiveBeginPlay`
  (bind _outactors (`GameplayStatics.GetAllActorsOfClass` "/Game/Robin/Hero/HeroCharacterBP.HeroCharacterBP_C"))
  (set `self.Player` (`KismetArrayLibrary.Array_Get` _outactors)))

(event `self.ReceiveTick`
  (params (DeltaSeconds :type "Float (single-precision)"))
  (bind _player (`self.Player`))
  (bind _player_2 (`self.Player`))
  (bind _defaultsceneroot (`self.DefaultSceneRoot`))
  (bind _returnvalue (`KismetMathLibrary.MakeVector` (.x (`SceneComponent.K2_GetComponentLocation` _defaultsceneroot)) (.y (`SceneComponent.K2_GetComponentLocation` _defaultsceneroot))))
  (bind _returnvalue_2 (`KismetMathLibrary.MakeVector` (.x (`SceneComponent.K2_GetComponentLocation` (`Character.CapsuleComponent` _player))) (.y (`SceneComponent.K2_GetComponentLocation` (`Character.CapsuleComponent` _player)))))
  (if (`/Game/Robin/Hero/HeroCharacterBP.InMenu` _player)
    (if (== (`/Game/Robin/Hero/HeroCharacterBP.Menu` _player) self)
      (if (> (`KismetMathLibrary.VSize` (- _returnvalue_2 _returnvalue)) 10.0)
        (`Pawn.AddMovementInput` _player_2 (`KismetMathLibrary.GetDirectionVector` _returnvalue_2 _returnvalue) 1.0 false)
        (goto _label :!via `Reset`)
        (else
          (`/Engine/EditorBlueprintResources/StandardMacros.DoOnce` false :!label _label
            (:`Completed`
              (`self.SetActorRotation` _player_2 (`SceneComponent.K2_GetComponentRotation` _defaultsceneroot)))))))))

(event `self.OpenMenu`
  (bind _player (`self.Player`))
  (`PlayerController.SetViewTargetWithBlend` (`GameplayStatics.GetPlayerController` 0) (`/Game/Robin/Hero/HeroCharacterBP.MenuCamera` _player) 0.5 "VTBlend_Linear" 0.0 true)
  (set `/Game/Robin/Hero/HeroCharacterBP.InMenu` true _player)
  (goto _label :!via `Reset`))

(event `self.Exit`
  (params (Pressed :type Boolean) (Key :type "Key Structure" :default "AnyKey"))
  (bind _player (`self.Player`))
  (if Pressed
    (if (`/Game/Robin/Hero/HeroCharacterBP.Sleeping` _player)
      (set `/Game/Robin/Hero/HeroCharacterBP.Sleeping` false _player))
    (set `/Game/Robin/Hero/HeroCharacterBP.InMenu` false _player)))

(event `self.Jump`
  (params (Pressed :type Boolean) (Key :type "Key Structure" :default "AnyKey"))
  (bind _player (`self.Player`))
  (if Pressed
    (bind _output_get (set `/Game/Robin/Hero/HeroCharacterBP.Sleeping` (not (`/Game/Robin/Hero/HeroCharacterBP.Sleeping` _player)) _player))
    (if (not _output_get)
      (set `/Game/Robin/Hero/HeroCharacterBP.InMenu` false _player))))

(fn `UserConstructionScript`)