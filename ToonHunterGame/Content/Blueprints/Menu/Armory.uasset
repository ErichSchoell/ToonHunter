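; Armory cabinet Blueprint for the menu, with left and right doors that swing open and closed.
; The Open and Close events take DeltaSeconds and rotate both doors incrementally in mirrored directions, at a speed scaled by the Time variable.
; Only the right door's relative yaw is checked against the open and closed limits, and the file has no Tick or timeline driving the events.
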(event `Open`
  (params (DeltaSeconds :type "Float (double-precision)"))
  (bind (_relativerotation_roll _relativerotation_pitch _relativerotation_yaw) (`KismetMathLibrary.BreakRotator` (`SceneComponent.RelativeRotation` (`self.Schrank_Tür_Rechts`))))
  (bind _returnvalue (`KismetMathLibrary.MakeRotator` 0.0 0.0 (/ (* DeltaSeconds -120.0) (`self.Time`))))
  ;[1 1 1] Open
  (if (> _relativerotation_yaw -120.0)
    (`SceneComponent.K2_AddRelativeRotation` (`self.Schrank_Tür_Rechts`) _returnvalue false false)
    (`SceneComponent.K2_AddRelativeRotation` (`self.Schran_Tür_Links`) (* _returnvalue -1) false false)))

(event `Close`
  (params (DeltaSeconds :type "Float (double-precision)"))
  (bind (_relativerotation_roll _relativerotation_pitch _relativerotation_yaw) (`KismetMathLibrary.BreakRotator` (`SceneComponent.RelativeRotation` (`self.Schrank_Tür_Rechts`))))
  (bind _returnvalue (`KismetMathLibrary.MakeRotator` 0.0 0.0 (/ (* DeltaSeconds 120.0) (`self.Time`))))
  ;[1 1 1] Close
  (if (< _relativerotation_yaw 0.0)
    (`SceneComponent.K2_AddRelativeRotation` (`self.Schrank_Tür_Rechts`) _returnvalue false false)
    (`SceneComponent.K2_AddRelativeRotation` (`self.Schran_Tür_Links`) (* _returnvalue -1) false false)))

(fn `UserConstructionScript`)