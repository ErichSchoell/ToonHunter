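; Inventory menu actor with two lid components, DeckelL and DeckelR, that swing open on their own.
; Tick adds a fixed roll step to both lids each frame until the left lid's roll reaches about -120 degrees, so the speed depends on frame rate.
; A mirrored close branch that rolls the lids back toward zero exists but is unconnected and never runs.
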(event `self.ReceiveBeginPlay`)

(event `self.ReceiveActorBeginOverlap`
  (params (OtherActor :type "Actor Object Reference")))

(event `self.ReceiveTick`
  (params (DeltaSeconds :type "Float (single-precision)"))
  (bind _relativerotation_roll (`KismetMathLibrary.BreakRotator` (`SceneComponent.RelativeRotation` (`self.Deckel_L`))))
  ;[1 1 1] Open
  (if (> _relativerotation_roll -120.0)
    (`SceneComponent.K2_AddRelativeRotation` (`self.Deckel_L`) (struct :`Roll` -1.0) false false)
    (`SceneComponent.K2_AddRelativeRotation` (`self.Deckel_R`) (struct :`Roll` -1.0) false false)))

(fn `UserConstructionScript`)