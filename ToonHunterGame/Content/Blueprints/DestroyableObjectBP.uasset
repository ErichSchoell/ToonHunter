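; DestroyableObjectBP is an actor that loses durability from specific damage types and is destroyed when it runs out.
; On AnyDamage it steps through the DamagableBy array with a looped branch until the damage type's class matches.
; A match subtracts truncated damage from Durability, prints a debug message and destroys the actor below one.
; The Index counter is never reset, so each search resumes where the last stopped.
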(event `self.ReceiveBeginPlay`)

(event `self.ReceiveActorBeginOverlap`
  (params (OtherActor :type "Actor Object Reference")))

(event `self.ReceiveTick`
  (params (DeltaSeconds :type "Float (single-precision)")))

(event `self.ReceiveAnyDamage`
  (params (Damage :type "Float (single-precision)") (DamageType :type "DamageType Object Reference") (InstigatedBy :type "Controller Object Reference") (DamageCauser :type "Actor Object Reference"))
  (bind _damagable_by (`self.Damagable By`))
  (bind _index (`self.index`))
  (if (== (`GameplayStatics.GetObjectClass` DamageType) (`KismetArrayLibrary.Array_Get` _damagable_by _index)) :!label _label
    (bind _output_get (set `self.Durability` (- (`self.Durability`) (`KismetMathLibrary.FTrunc` Damage))))
    (`KismetSystemLibrary.PrintString` (`KismetStringLibrary.JoinStringArray` (`|MakeArray` "There was" (`KismetStringLibrary.Conv_DoubleToString` Damage) "Dealt from type" (`KismetSystemLibrary.GetDisplayName` DamageType) "by" (`KismetSystemLibrary.GetDisplayName` InstigatedBy) "with" (`KismetSystemLibrary.GetDisplayName` DamageCauser))) true true (struct :`G` 0.66 :`B` 1.0 :`A` 1.0) 4.0)
    (if (< _output_get 1)
      (`self.K2_DestroyActor`))
    (else
      (set `self.index` (+ _index 1))
      (if (< _index (`KismetArrayLibrary.Array_Length` _damagable_by))
        (goto _label)))))

(fn `UserConstructionScript`)