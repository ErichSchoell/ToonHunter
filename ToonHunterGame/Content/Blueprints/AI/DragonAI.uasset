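; DragonAI is the AI controller logic for a dragon that treats the player as its enemy.
; On BeginPlay it seeds Monster_Blackboard with a home path node, player location and enemy, then starts DragonBT after a short delay.
; AI Perception updates enemy visibility from the first sensed stimulus.
; Tick copies the enemy's location to the blackboard while visible and continually mirrors the TakenDamage flag.
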(event `self.ReceiveBeginPlay`
  (bind _homepathnode (`self.HomePathNode`))
  (bind _blackboardcomponent (`self.UseBlackboard` "/Game/Blueprints/AI/Monster_Blackboard.Monster_Blackboard"))
  (set `self.MyBlackboard` _blackboardcomponent)
  (`|ExecutionSequence`
    (:`then_0`
      (`BlackboardComponent.SetValueAsObject` (`self.MyBlackboard`) (`self.BKeyHomePathNode`) _homepathnode)
      (set `self.NextPathNode` _homepathnode)
      (`BlackboardComponent.SetValueAsObject` (`self.MyBlackboard`) (`self.BKeyNextPathNode`) (`self.NextPathNode`))
      (set `self.SuggestedLocation` (`self.K2_GetActorLocation` (`GameplayStatics.GetPlayerPawn` 0)))
      (`BlackboardComponent.SetValueAsVector` (`self.MyBlackboard`) (`self.BKeySuggestedLocation`) (`self.SuggestedLocation`)))
    (:`then_1`
      (`self.SetEnemy` (`GameplayStatics.GetPlayerPawn` 0))
      (`KismetSystemLibrary.Delay` 0.1)
      (`self.RunBehaviorTree` "/Game/Blueprints/AI/DragonBT.DragonBT"))))

(event `self.AIPerception.OnPerceptionUpdated`
  (params (UpdatedActors :type "Array of Actor Object Reference"))
  (for _array_element UpdatedActors
    (if (== _array_element (`self.Enemy`))
      (`self.UpdatePerception` (`self.AIPerception`) _array_element)
      (`BlackboardComponent.SetValueAsBool` (`self.MyBlackboard`) (`self.BKeyIsEnemyVisible`) (`self.IsEnemyVisible`)))))

(event `self.ReceiveTick`
  (params (DeltaSeconds :type "Float (single-precision)"))
  (`|ExecutionSequence`
    (:`then_0`
      (if (`self.IsEnemyVisible`)
        (set `self.SuggestedLocation` (`self.K2_GetActorLocation` (`self.Enemy`)))
        (`BlackboardComponent.SetValueAsVector` (`self.MyBlackboard`) (`self.BKeySuggestedLocation`) (`self.SuggestedLocation`))))
    (:`then_1`
      (`BlackboardComponent.SetValueAsBool` (`self.MyBlackboard`) (`self.BKeyTakenDamage`) (`self.TakenDamage`)))))

(fn `SetEnemy`
  (params (NewEnemy :type "Actor Object Reference"))
  (if (!= NewEnemy (`self.Enemy`))
    (bind _output_get (set `self.Enemy` NewEnemy))
    (`BlackboardComponent.SetValueAsObject` (`AIBlueprintHelperLibrary.GetBlackboard` null) (`self.BKeyEnemy`) _output_get)
    (`self.UpdatePerception` (`self.AIPerception`) (`self.Enemy`))))

(fn `UpdatePerception`
  (params (PerceptionComponent :type "AIPerceptionComponent Object Reference") (EnemyActor :type "Actor Object Reference"))
  (bind _info (`AIPerceptionComponent.GetActorsPerception` PerceptionComponent EnemyActor))
  (bind (_target _lastsensedstimuli) (break `ActorPerceptionBlueprintInfo` _info))
  (if (>= (`KismetArrayLibrary.Array_Length` _lastsensedstimuli) 1)
    (set `self.IsEnemyVisible` (`.bSuccessfullySensed` (break `AIStimulus` (`KismetArrayLibrary.Array_Get` _lastsensedstimuli)))))
  (return))

(fn `UserConstructionScript`)