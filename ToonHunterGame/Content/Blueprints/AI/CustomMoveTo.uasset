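; Behavior tree task that walks the dragon character to a blackboard Target location on the horizontal plane.
; On execute it sets the character's max walk speed and derives a smoothing radius just beyond the acceptable radius.
; Each tick it steers straight at the target with movement input rather than pathfinding, easing input down linearly inside the smoothing radius.
; It finishes successfully near the acceptable radius and prints debug strings.
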(event EventReceiveTickAI
  (params (OwnerController :type AI%20Controller%20Object%20Reference) (ControlledPawn :type Pawn%20Object%20Reference) (DeltaSeconds :type Float%20%28single-precision%29))
  (bind _returnvalue (Transformation|GetActorLocation ControlledPawn))
  (bind _smoothingradius (Variables|Default|GetSmoothingRadius))
  (bind _smoothingradius_2 (Variables|Default|GetSmoothingRadius))
  (bind _acceptableradius (Variables|Default|GetAcceptableRadius))
  (bind _target (Variables|Default|GetTarget))
  (bind _returnvalue_2 (Class|BTFunctionLibrary|GetBlackboardValueasVector _target))
  (bind _returnvalue_3 (- _returnvalue_2 _returnvalue))
  (bind _returnvalue_4 (Math|Vector|MakeVector (.x _returnvalue_3) (.y _returnvalue_3) 0.0))
  (bind _returnvalue_5 (Math|Vector|VectorLength _returnvalue_4))
  (bind _returnvalue_6 (> _returnvalue_5 _smoothingradius))
  (bind _returnvalue_7 (|(max(((a-b)/(c-b)),0)) _returnvalue_5 _acceptableradius _smoothingradius_2))
  (bind _returnvalue_8 (select _returnvalue_6 1.0 _returnvalue_7))
  (if (< (- _returnvalue_5 1.0) (Variables|Default|GetAcceptableRadius))
    (Development|PrintString "Finished" true true "(R=0.000000,G=0.660000,B=1.000000,A=1.000000)" 0.0)
    (AI|BehaviorTree|FinishExecute true)
    (else
      (Development|PrintString (Utilities|String|ToString(Float) _returnvalue_8) true true "(R=0.000000,G=0.660000,B=1.000000,A=1.000000)" DeltaSeconds)
      (Pawn|Input|AddMovementInput ControlledPawn (Math|Vector|Normalize _returnvalue_4) _returnvalue_8 false))))

(event EventReceiveExecuteAI
  (params (OwnerController :type AI%20Controller%20Object%20Reference) (ControlledPawn :type Pawn%20Object%20Reference))
  (bind _asdragon_character_bp (Utilities|Casting|CastToDragonCharacterBP ControlledPawn))
  (Variables|/Script/Engine.CharacterMovementComponent|SetMaxWalkSpeed (Variables|/Script/Engine.Character|GetCharacterMovement _asdragon_character_bp) (Variables|Default|GetWalkSpeed))
  (Variables|Default|SetSmoothingRadius (+ (Variables|Default|GetAcceptableRadius) 5e+01)))