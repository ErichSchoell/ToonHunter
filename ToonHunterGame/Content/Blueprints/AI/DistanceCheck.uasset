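; Behavior tree decorator that passes when the AI pawn's distance to a target lies within a range.
; It overrides the AI condition check, reads the Target location from the blackboard as a vector and measures the straight-line 3D distance from the controlled pawn.
; The check returns true only when that distance is strictly between the Min and Max variables.
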(fn `PerformConditionCheckAI`
  (params (OwnerController :type "AIController Object Reference") (ControlledPawn :type "Pawn Object Reference"))
  (returns (ReturnValue :type Boolean))
  (bind _returnvalue (`KismetMathLibrary.VSize` (- (`Actor.K2_GetActorLocation` ControlledPawn) (`BTFunctionLibrary.GetBlackboardValueAsVector` (`self.Target`)))))
  (if (and (> _returnvalue (`self.Min`)) (< _returnvalue (`self.Max`)))
    (return true)
    (else
      (return false))))