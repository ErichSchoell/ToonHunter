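; Behavior tree task that makes a DragonCharacterBP pawn circle its blackboard Target in a randomly chosen direction.
; GetPointOnCircle finds the pawn's angle around the target and steps it by a fixed increment at the given radius to produce the next waypoint.
; Tick maintains walk speed and requests another waypoint through a gate whenever the pawn nears its goal in 2D.
; The task runs until aborted, which closes the gate and halts the pawn.
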(event EventReceiveAbortAI
  (params (OwnerController :type AI%20Controller%20Object%20Reference) (ControlledPawn :type Pawn%20Object%20Reference))
  (Utilities|FlowControl|Sequence
    (:then_0
      (Utilities|FlowControl|Gate false) ; enters at Close
    )
    (:then_1
      (bind _output_get (Variables|Default|SetGoal (Transformation|GetActorLocation ControlledPawn)))
      (AI|AIMoveTo ControlledPawn _output_get 0 1e+01 false
        (:then
          (Class|BTTaskBlueprintBase|FinishAbort))))))

(event EventReceiveTickAI
  (params (OwnerController :type AI%20Controller%20Object%20Reference) (ControlledPawn :type Pawn%20Object%20Reference) (DeltaSeconds :type Float%20%28single-precision%29))
  (bind _returnvalue (Transformation|GetActorLocation ControlledPawn))
  (bind _walkspeed (Variables|Default|GetWalkSpeed))
  (Utilities|FlowControl|Sequence
    (:then_0
      ;[1 1 1] Set WalkSpeed
      (bind _asdragon_character_bp (Utilities|Casting|CastToDragonCharacterBP ControlledPawn))
      (if (!= (Variables|/Script/Engine.CharacterMovementComponent|GetMaxWalkSpeed (Variables|/Script/Engine.Character|GetCharacterMovement _asdragon_character_bp)) _walkspeed)
        (Variables|/Script/Engine.CharacterMovementComponent|SetMaxWalkSpeed (Variables|/Script/Engine.Character|GetCharacterMovement _asdragon_character_bp) (Math|Interpolation|FInterpTo (Variables|/Script/Engine.CharacterMovementComponent|GetMaxWalkSpeed (Variables|/Script/Engine.Character|GetCharacterMovement _asdragon_character_bp)) _walkspeed DeltaSeconds 5.0))))
    (:then_1
      ;[1 1 1] Distance Check
      (if (<= (Math|Vector|VectorLength (- (Math|Vector|MakeVector (.x _returnvalue) (.y _returnvalue) 0.0) (Math|Vector|MakeVector (.x (Variables|Default|GetGoal)) (.y (Variables|Default|GetGoal)) 0.0))) 5e+01)
        (Utilities|FlowControl|Gate false
          (:Exit
            (bind _circlepoint (CallFunction|GetPointonCircle (Transformation|GetActorLocation (stale EventReceiveExecuteAI ControlledPawn)) (Class|BTFunctionLibrary|GetBlackboardValueasVector (Variables|Default|GetTarget)) (Variables|Default|GetRadius) (Variables|Default|GetAngleBetweenWaypoints) (Variables|Default|GetClockwise)))
            (bind _output_get (Variables|Default|SetGoal _circlepoint))
            (AI|AIMoveTo (stale EventReceiveExecuteAI ControlledPawn) (Variables|Default|GetGoal) 0 0.0 false)))))))

(event EventReceiveExecuteAI
  (params (OwnerController :type AI%20Controller%20Object%20Reference) (ControlledPawn :type Pawn%20Object%20Reference))
  (bind _asdragon_character_bp (Utilities|Casting|CastToDragonCharacterBP ControlledPawn))
  (Variables|/Script/Engine.CharacterMovementComponent|SetMaxWalkSpeed (Variables|/Script/Engine.Character|GetCharacterMovement _asdragon_character_bp) (Variables|Default|GetWalkSpeed))
  (Utilities|FlowControl|Sequence
    (:then_0
      (goto _label Open))
    (:then_1
      (Variables|Default|SetClockwise (Math|Random|RandomBool))
      (Utilities|FlowControl|Gate false :!label _label
        (:Exit
          (bind _circlepoint (CallFunction|GetPointonCircle (Transformation|GetActorLocation ControlledPawn) (Class|BTFunctionLibrary|GetBlackboardValueasVector (Variables|Default|GetTarget)) (Variables|Default|GetRadius) (Variables|Default|GetAngleBetweenWaypoints) (Variables|Default|GetClockwise)))
          (bind _output_get (Variables|Default|SetGoal _circlepoint))
          (AI|AIMoveTo ControlledPawn (Variables|Default|GetGoal) 0 0.0 false))))))

(fn GetPointonCircle
  (params (This :type Vector) (Target :type Vector) (Radius :type Float%20%28single-precision%29) (AngleBetweenPoints :type Float%20%28single-precision%29) (Clockwise :type Boolean))
  (bind (_x _y) (Math|Vector|BreakVector Target))
  (Utilities|FlowControl|Sequence
    (:then_0
      ;[1 1 1] Set Local Variables
      (LocalVariables|SetLocal_CenterX _x)
      (LocalVariables|SetLocal_CenterY _y)
      (LocalVariables|SetLocal_Radius Radius)
      (LocalVariables|SetLocal_AngleBetweenPoints AngleBetweenPoints))
    (:then_1
      ;[1 1 1] Get Starting Angle
      (LocalVariables|SetLocal_Angle (* (Class|KismetMathLibrary|DegAcos (Math|Vector|DotProduct (Math|Vector|Normalize (- This Target)) (Math|Vector|GetForwardVector "0,0.000000, 0"))) (select (> (.Y (Math|Vector|BreakVector This)) (.Y (Math|Vector|BreakVector Target))) 1.0 -1.0))))
    (:then_2
      ;[1 1 1] Set Points on Circle
      (bind _output_get (LocalVariables|SetLocal_CirclePoints (Math|Vector|MakeVector (+ (LocalVariables|GetLocal_CenterX) (* (LocalVariables|GetLocal_Radius) (Math|Trig|Cos(Degrees) (select Clockwise (+ (LocalVariables|GetLocal_Angle) (LocalVariables|GetLocal_AngleBetweenPoints)) (- (LocalVariables|GetLocal_Angle) (LocalVariables|GetLocal_AngleBetweenPoints)))))) (+ (LocalVariables|GetLocal_CenterY) (* (LocalVariables|GetLocal_Radius) (Math|Trig|Sin(Degrees) (select Clockwise (+ (LocalVariables|GetLocal_Angle) (LocalVariables|GetLocal_AngleBetweenPoints)) (- (LocalVariables|GetLocal_Angle) (LocalVariables|GetLocal_AngleBetweenPoints)))))) 0.0)))
      (return _output_get))))