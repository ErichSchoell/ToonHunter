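; Dragon enemy character that hands its home path node to DragonAI and tracks its own health, shown as debug text.
; A head-socket damage area, enabled only while the anim Blueprint is attacking, knocks back the hero, turns it toward the dragon and applies damage.
; Damage taken lowers health and flags the anim Blueprint.
; Tick also derives a smoothed animation turn speed by dotting the right vector with a delayed forward vector.
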(event `self.ReceiveBeginPlay`
  (set `self.CurrentHealth` (`self.MaxHealth`))
  (bind _returnvalue (`AIBlueprintHelperLibrary.GetAIController` self))
  (bind _asdragon_ai (cast `/Game/Blueprints/AI/DragonAI` _returnvalue))
  (set `self.MonsterAI` _asdragon_ai)
  (bind _output_get (set `/Game/Blueprints/AI/DragonAI.HomePathNode` (`self.HomePathNode`) (`self.MonsterAI`)))
  (set `/Game/Blueprints/AI/DragonAI.NextPathNode` _output_get (`self.MonsterAI`)))

(event `self.DamageArea1.OnComponentBeginOverlap`
  (params (OtherActor :type "Actor Object Reference") (OtherComp :type "PrimitiveComponent Object Reference") (OtherBodyIndex :type Integer) (bFromSweep :type Boolean) (SweepResult :type "HitResult Structure (by ref)"))
  (bind _returnvalue (`self.K2_GetActorLocation` OtherActor))
  (bind _returnvalue_2 (`SceneComponent.K2_GetComponentLocation` (`self.CapsuleComponent`)))
  (bind (_returnvalue_x _returnvalue_y) (`KismetMathLibrary.BreakVector` (`KismetMathLibrary.GetDirectionVector` _returnvalue_2 _returnvalue)))
  (bind _ashero_character_bp (cast `/Game/Robin/Hero/HeroCharacterBP` OtherActor))
  (`KismetSystemLibrary.RetriggerableDelay` 0.05) ; To prevent multiple collsion detections at once
  (`CharacterMovementComponent.AddImpulse` (`Character.CharacterMovement` _ashero_character_bp) (* (`KismetMathLibrary.MakeVector` _returnvalue_x _returnvalue_y 0.5) 50000.0) false)
  (`self.SetActorRotation` OtherActor (`KismetMathLibrary.FindLookAtRotation` _returnvalue _returnvalue_2))
  (`GameplayStatics.ApplyDamage` OtherActor 1.0))

(event `self.ReceiveAnyDamage`
  (params (Damage :type "Float (single-precision)") (DamageType :type "DamageType Object Reference") (InstigatedBy :type "Controller Object Reference") (DamageCauser :type "Actor Object Reference"))
  (set `self.CurrentHealth` (- (`self.CurrentHealth`) Damage))
  (bind _asdragon_anim_bp (cast `/Game/Animations/Dragon/Dragon_AnimBP` (`SkeletalMeshComponent.GetAnimInstance` (`self.Mesh`))))
  (set `/Game/Animations/Dragon/Dragon_AnimBP.TakenDamage` true _asdragon_anim_bp))

(event `self.ReceiveTick`
  (params (DeltaSeconds :type "Float (single-precision)"))
  (bind _damagearea1 (`self.DamageArea1`))
  (`|ExecutionSequence`
    (:`then_0`
      (`KismetSystemLibrary.PrintString` (`KismetStringLibrary.Concat_StrStr` "Monster Health: " (`KismetStringLibrary.Conv_IntToString` (`KismetMathLibrary.FFloor` (`self.CurrentHealth`))) "/" (`KismetStringLibrary.Conv_IntToString` (`KismetMathLibrary.FFloor` (`self.MaxHealth`)))) true false (struct :`R` 0.386461 :`B` 0.685 :`A` 1.0) (`GameplayStatics.GetWorldDeltaSeconds`)))
    (:`then_1`
      (bind _asdragon_anim_bp (cast `/Game/Animations/Dragon/Dragon_AnimBP` (`SkeletalMeshComponent.GetAnimInstance` (`self.Mesh`))))
      (`|ExecutionSequence`
        (:`then_0`
          ;[1 1 1] Toggle DamageArea when attacking
          (if (`/Game/Animations/Dragon/Dragon_AnimBP.Attack` _asdragon_anim_bp)
            (`PrimitiveComponent.SetCollisionEnabled` _damagearea1 "QueryAndPhysics")
            (else
              (`PrimitiveComponent.SetCollisionEnabled` _damagearea1 "NoCollision"))))
        (:`then_1`
          ;[1 1 1] Set TurnSpeed
          (`|ExecutionSequence`
            (:`then_0`
              (`KismetSystemLibrary.Delay` 0.1)
              (set `self.TagetTurnSpeed` (* (`KismetMathLibrary.Dot_VectorVector` (`self.GetActorRightVector`) (`self.LastForward`)) 100.0))
              (set `self.LastForward` (`self.GetActorForwardVector`)))
            (:`then_1`
              (set `/Game/Animations/Dragon/Dragon_AnimBP.TurnSpeed` (`KismetMathLibrary.FInterpTo` (`/Game/Animations/Dragon/Dragon_AnimBP.TurnSpeed` _asdragon_anim_bp) (`self.TagetTurnSpeed`) (`GameplayStatics.GetWorldDeltaSeconds`) 10.0) _asdragon_anim_bp))))))))

(fn `UserConstructionScript`
  (`SceneComponent.K2_AttachTo` (`self.DamageArea1`) (`self.Mesh`) "headSocket" "SnapToTarget" true))