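; Behavior tree service that decides when an AI_Character should retreat based on its health.
; Each tick it sets the NeedToRetreat blackboard key to whether the health ratio is at or below RetreatThreshold.
; When it is, the service halves that threshold, so subsequent retreats require lower health.
; It then sets NeedToRetreatHome by comparing the halved threshold to a tenth of MaxHealth, rather than to a ratio.
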(event `self.ReceiveTickAI`
  (params (OwnerController :type "AIController Object Reference") (ControlledPawn :type "Pawn Object Reference") (DeltaSeconds :type "Float (single-precision)"))
  (bind _asai_character (cast `/Game/Blueprints/AI/AI_Character` ControlledPawn))
  (bind _returnvalue (<= (/ (`/Game/Blueprints/AI/AI_Character.CurrentHealth` _asai_character) (`/Game/Blueprints/AI/AI_Character.MaxHealth` _asai_character)) (`/Game/Blueprints/AI/AI_Character.RetreatThreshold` _asai_character)))
  (`BTFunctionLibrary.SetBlackboardValueAsBool` (`self.NeedToRetreat_Key`) _returnvalue)
  (if _returnvalue
    (bind _output_get (set `/Game/Blueprints/AI/AI_Character.RetreatThreshold` (/ (`/Game/Blueprints/AI/AI_Character.RetreatThreshold` _asai_character) 2.0) _asai_character))
    (`BTFunctionLibrary.SetBlackboardValueAsBool` (`self.NeedToRetreatHome_Key`) (<= _output_get (/ (`/Game/Blueprints/AI/AI_Character.MaxHealth` _asai_character) 10.0)))))