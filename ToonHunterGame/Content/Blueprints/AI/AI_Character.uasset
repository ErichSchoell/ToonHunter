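; AI monster character Blueprint with a dragon animation Blueprint, handling its health, flinching and head attack.
; On BeginPlay it fills health and seeds its Monster_AI controller with home and next path nodes.
; A head-socket damage area, enabled each Tick while the animation's Attack flag is set, knocks back overlapping heroes and calls ApplyDamage.
; Taking damage lowers health, ends any attack and flags TakenDamage on the controller for FlinchTime.
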(event `self.ReceiveBeginPlay`
  (set `self.CurrentHealth` (`self.MaxHealth`))
  (bind _returnvalue (`AIBlueprintHelperLibrary.GetAIController` self))
  (bind _asmonster_ai (cast `/Game/Blueprints/AI/Monster_AI` _returnvalue))
  (set `self.MonsterAI` _asmonster_ai)
  (bind _output_get (set `/Game/Blueprints/AI/Monster_AI.HomePathNode` (`self.HomePathNode`) (`self.MonsterAI`)))
  (set `/Game/Blueprints/AI/Monster_AI.NextPathNode` _output_get (`self.MonsterAI`)))

(event `self.DamageArea1.OnComponentBeginOverlap`
  (params (OtherActor :type "Actor Object Reference") (OtherComp :type "PrimitiveComponent Object Reference") (OtherBodyIndex :type Integer) (bFromSweep :type Boolean) (SweepResult :type "HitResult Structure (by ref)"))
  (bind (_returnvalue_x _returnvalue_y) (`KismetMathLibrary.BreakVector` (`KismetMathLibrary.GetDirectionVector` (`SceneComponent.K2_GetComponentLocation` (`self.CapsuleComponent`)) (`self.K2_GetActorLocation` OtherActor))))
  (bind _ashero_character_bp (cast `/Game/Robin/Hero/HeroCharacterBP` OtherActor))
  (`KismetSystemLibrary.RetriggerableDelay` 0.05) ; To prevent multiple collsion detections at once
  (`CharacterMovementComponent.AddImpulse` (`Character.CharacterMovement` _ashero_character_bp) (* (`KismetMathLibrary.MakeVector` _returnvalue_x _returnvalue_y 0.5) 50000.0) false)
  (`KismetSystemLibrary.PrintString` "Hit" true false (struct :`R` 1.0 :`B` 0.006919 :`A` 1.0))
  (`GameplayStatics.ApplyDamage` null 1.0))

(event `self.ReceiveAnyDamage`
  (params (Damage :type "Float (single-precision)") (DamageType :type "DamageType Object Reference") (InstigatedBy :type "Controller Object Reference") (DamageCauser :type "Actor Object Reference"))
  (set `self.CurrentHealth` (- (`self.CurrentHealth`) Damage))
  (bind _asdragon_anim_bp (cast `/Game/Animations/Dragon/Dragon_AnimBP` (`SkeletalMeshComponent.GetAnimInstance` (`self.Mesh`))))
  (`/Game/Animations/Dragon/Dragon_AnimBP.AnimNotify_AttackEnd` _asdragon_anim_bp)
  (set `/Game/Blueprints/AI/Monster_AI.TakenDamage` true (`self.MonsterAI`))
  (`KismetSystemLibrary.RetriggerableDelay` (`self.FlinchTime`))
  (set `/Game/Blueprints/AI/Monster_AI.TakenDamage` false (`self.MonsterAI`)))

(event `self.ReceiveTick`
  (params (DeltaSeconds :type "Float (single-precision)"))
  (bind _damagearea1 (`self.DamageArea1`))
  (`|ExecutionSequence`
    (:`then_0`
      (`KismetSystemLibrary.PrintString` (`KismetStringLibrary.Concat_StrStr` "Monster Health: " (`KismetStringLibrary.Conv_IntToString` (`KismetMathLibrary.FFloor` (`self.CurrentHealth`))) "/" (`KismetStringLibrary.Conv_IntToString` (`KismetMathLibrary.FFloor` (`self.MaxHealth`)))) true true (struct :`R` 0.386461 :`B` 0.685 :`A` 1.0) (`GameplayStatics.GetWorldDeltaSeconds`)))
    (:`then_1`
      (bind _asdragon_anim_bp (cast `/Game/Animations/Dragon/Dragon_AnimBP` (`SkeletalMeshComponent.GetAnimInstance` (`self.Mesh`))))
      (if (`/Game/Animations/Dragon/Dragon_AnimBP.Attack` _asdragon_anim_bp)
        (`PrimitiveComponent.SetCollisionEnabled` _damagearea1 "QueryAndPhysics")
        (`SceneComponent.SetHiddenInGame` _damagearea1 false false)
        (else
          (`PrimitiveComponent.SetCollisionEnabled` _damagearea1 "NoCollision")
          (`SceneComponent.SetHiddenInGame` _damagearea1 true false))))))

(fn `UserConstructionScript`
  (`SceneComponent.K2_AttachTo` (`self.DamageArea1`) (`self.Mesh`) "headSocket" "SnapToTarget" true))