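; SetRetreatLocation is a behavior tree task that computes a retreat point for the controlled pawn and writes it to the RetreatLocation blackboard key.
; It takes the direction from the pawn to the Target vector and yaws it randomly 10 to 30 degrees to either side.
; The point lies Distance along that direction from the pawn, so it falls toward Target unless Distance is negative.
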(event `self.ReceiveExecuteAI`
  (params (OwnerController :type "AIController Object Reference") (ControlledPawn :type "Pawn Object Reference"))
  (bind _returnvalue (`Actor.K2_GetActorLocation` ControlledPawn))
  (`BTFunctionLibrary.SetBlackboardValueAsVector` (`self.RetreatLocation`) (+ _returnvalue (* (`KismetMathLibrary.Normal` (`KismetMathLibrary.GreaterGreater_VectorRotator` (- (`BTFunctionLibrary.GetBlackboardValueAsVector` (`self.Target`)) _returnvalue) (`KismetMathLibrary.MakeRotator` 0.0 0.0 (select `bool` (`KismetMathLibrary.RandomBool`) :`false` (`KismetMathLibrary.RandomFloatInRange` -30.0 -10.0) :`true` (`KismetMathLibrary.RandomFloatInRange` 10.0 30.0))))) (`self.Distance`))))
  (`self.FinishExecute` true))