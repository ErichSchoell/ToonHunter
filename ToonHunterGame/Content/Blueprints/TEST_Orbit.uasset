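; Test Blueprint that lays out five markers (Start, 1, 2, 3, End) along a circular arc around Target in the construction script.
; NewFunction1 takes Enemy's signed bearing from Target against world X, then steps back by a fixed angle to build points at the given radius, with Z at zero.
; An older chain using the single-point NewFunction0 remains unconnected, and the event graph is empty.
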(event EventBeginPlay)

(event EventActorBeginOverlap
  (params (OtherActor :type Actor%20Object%20Reference)))

(event EventTick
  (params (DeltaSeconds :type Float%20%28single-precision%29)))

(fn ConstructionScript
  (bind _circlepoint (CallFunction|NewFunction1 (Transformation|GetWorldLocation (Variables|Default|GetTarget)) (Variables|Default|GetRadius) (Variables|Default|GetAngle) (Variables|Default|GetNumberOfPoints)))
  (Transformation|SetWorldLocation (Variables|Default|GetStart) (Utilities|Array|Get(acopy) _circlepoint) false false)
  (Transformation|SetWorldLocation (Variables|Default|Get1) (Utilities|Array|Get(acopy) _circlepoint 1) false false)
  (Transformation|SetWorldLocation (Variables|Default|Get2) (Utilities|Array|Get(acopy) _circlepoint 2) false false)
  (Transformation|SetWorldLocation (Variables|Default|Get3) (Utilities|Array|Get(acopy) _circlepoint 3) false false)
  (Transformation|SetWorldLocation (Variables|Default|GetEnd) (Utilities|Array|Get(acopy) _circlepoint 4) false false))

(fn NewFunction0
  (params (Center :type Vector) (Radius :type Float%20%28single-precision%29) (Angle :type Float%20%28single-precision%29))
  (return (Math|Vector|MakeVector (+ (.x Center) (* Radius (Math|Trig|Cos(Degrees) Angle))) (+ (.y Center) (* Radius (Math|Trig|Sin(Degrees) Angle))) (.z Center))))

(fn NewFunction1
  (params (Center :type Vector) (Radius :type Float%20%28single-precision%29) (AngleBetweenPoints :type Float%20%28single-precision%29) (NumberOfPoints :type Integer))
  (bind _target (Variables|Default|GetTarget))
  (bind _enemy (Variables|Default|GetEnemy))
  (bind _returnvalue (Transformation|GetWorldLocation _enemy))
  (bind _returnvalue_2 (Transformation|GetWorldLocation _target))
  (Utilities|FlowControl|Sequence
    (:then_0
      ;[1 1 1] Set Local Variables
      (LocalVariables|SetLocal_CenterX (.x Center))
      (LocalVariables|SetLocal_CenterY (.y Center))
      (LocalVariables|SetLocal_Radius Radius)
      (LocalVariables|SetLocal_AngleBetweenPoints AngleBetweenPoints)
      (LocalVariables|SetLocal_NumberOfPoints NumberOfPoints))
    (:then_1
      ;[1 1 1] Get Starting Angle
      (LocalVariables|SetLocal_Angle (* (Class|KismetMathLibrary|DegAcos (Math|Vector|DotProduct (Math|Vector|Normalize (- _returnvalue _returnvalue_2)) (Math|Vector|GetForwardVector "0,0.000000, 0"))) (select (> (.Y (Math|Vector|BreakVector _returnvalue)) (.Y (Math|Vector|BreakVector _returnvalue_2))) 1.0 -1.0))))
    (:then_2
      ;[1 1 1] Set Points on Circle
      (for _index (range 1 (LocalVariables|GetLocal_NumberOfPoints))
        (Utilities|Array|Add (LocalVariables|GetLocal_CirclePoints) (Math|Vector|MakeVector (+ (LocalVariables|GetLocal_CenterX) (* (LocalVariables|GetLocal_Radius) (Math|Trig|Cos(Degrees) (- (LocalVariables|GetLocal_Angle) (* _index (LocalVariables|GetLocal_AngleBetweenPoints)))))) (+ (LocalVariables|GetLocal_CenterY) (* (LocalVariables|GetLocal_Radius) (Math|Trig|Sin(Degrees) (- (LocalVariables|GetLocal_Angle) (* _index (LocalVariables|GetLocal_AngleBetweenPoints)))))) 0.0)))
      (return (LocalVariables|GetLocal_CirclePoints)))))